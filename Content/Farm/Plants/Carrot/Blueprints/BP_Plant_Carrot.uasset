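; Carrot plant actor for the farm that grows through four visual stages over time.
; A looping five-second timer started on BeginPlay advances GrowthStage up to the final stage, refreshes the visuals and prints a debug string.
; UpdatePlantVisual switches on the stage to scale the leaves and root meshes, hiding the root at stage zero and sinking it deeper as it grows.
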(event `self.ReceiveBeginPlay`
  (`self.UpdatePlantVisual`)
  (`KismetSystemLibrary.K2_SetTimerDelegate` (delegate `GrowTick`) 5.0 true))

(event `GrowTick`
  (if (< (`self.GrowthStage`) 3)
    (set `self.GrowthStage` (+ (`self.GrowthStage`) 1))
    (`self.UpdatePlantVisual`)
    (`KismetSystemLibrary.PrintString` "Hello")))

(fn `UpdatePlantVisual`
  (bind _leavesmesh (`self.LeavesMesh`))
  (bind _rootmesh (`self.RootMesh`))
  (switch `int` (`self.GrowthStage`)
    (:`0`
      (`SceneComponent.SetRelativeScale3D` _leavesmesh (0.05 0.05 0.05))
      (`SceneComponent.SetVisibility` _rootmesh false false))
    (:`1`
      (`SceneComponent.SetRelativeScale3D` _leavesmesh (0.08 0.08 0.12))
      (`SceneComponent.SetRelativeScale3D` _rootmesh (0.15 0.15 0.25))
      (`SceneComponent.SetVisibility` _rootmesh true false)
      (`SceneComponent.K2_SetRelativeLocation` _rootmesh (0.0 0.0 -8.0) false false))
    (:`2`
      (`SceneComponent.SetRelativeScale3D` _leavesmesh (0.12 0.12 0.2))
      (`SceneComponent.SetRelativeScale3D` _rootmesh (0.22 0.22 0.45))
      (`SceneComponent.SetVisibility` _rootmesh true false)
      (`SceneComponent.K2_SetRelativeLocation` _rootmesh (0.0 0.0 -14.0) false false))
    (:`3`
      (`SceneComponent.SetRelativeScale3D` _leavesmesh (0.18 0.18 0.3))
      (`SceneComponent.SetRelativeScale3D` _rootmesh (0.3 0.3 0.65))
      (`SceneComponent.SetVisibility` _rootmesh true false)
      (`SceneComponent.K2_SetRelativeLocation` _rootmesh (0.0 0.0 -20.0) false false))))

(fn `UserConstructionScript`)