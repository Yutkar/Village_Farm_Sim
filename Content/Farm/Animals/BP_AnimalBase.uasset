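; Base farm animal Blueprint that simulates aging, hunger and death.
; A looping timer from BeginPlay drives DecreaseNeeds, which advances age, drains hunger, prints a debug readout and damages health while starving.
; CheckGrowth maps age to a life stage (Baby, Teenager, Adult, Elderly) and scales the capsule to match.
; At zero health it stops AI logic, disables movement and turns on capsule physics; a Ragdoll profile call is left unconnected.
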(event `DecreaseNeeds`
  (bind _returnvalue (`AIBlueprintHelperLibrary.GetAIController` null))
  (set `self.Age` (+ (`self.Age`) 1.0))
  (`self.CheckGrowth`)
  (bind _output_get (set `self.Hunger` (`KismetMathLibrary.FClamp` (- (`self.Hunger`) 1.0) 0.0 100.0)))
  (`KismetSystemLibrary.PrintString` (`KismetTextLibrary.Conv_TextToString` (`|FormatText` "Голод: {H} | ХП: {Health}" _output_get (stale _output_get_2))) true true (struct :`R` 0.070542 :`G` 1.0 :`A` 1.0) 4.0)
  (if (<= (`self.Hunger`) 0.0)
    (bind _output_get_2 (set `self.Health` (`KismetMathLibrary.FClamp` (- (`self.Health`) 5.0) 0.0 100.0)))
    (if (<= (`self.Health`) 0.0)
      (`/Engine/EditorBlueprintResources/StandardMacros.IsValid` _returnvalue
        (:`Is Valid`
          (`BrainComponent.StopLogic` (`AIController.BrainComponent` _returnvalue) ""))
        (:`Is Not Valid`
          _))
      (`CharacterMovementComponent.DisableMovement` (`self.CharacterMovement`))
      (`PrimitiveComponent.SetSimulatePhysics` (`self.CapsuleComponent`) true)
      (`PrimitiveComponent.SetCollisionEnabled` (`self.CapsuleComponent`) "QueryAndPhysics"))))

(event `self.ReceiveBeginPlay`
  (`KismetSystemLibrary.K2_SetTimerDelegate` (delegate `DecreaseNeeds`) 5.0 true))

(fn `CheckGrowth`
  (bind _age (`self.Age`))
  (bind _capsulecomponent (`self.CapsuleComponent`))
  (if (< _age 10.0)
    (set `self.CurrentStage` "NewEnumerator0")
    (elif (< _age 20.0)
      (set `self.CurrentStage` "NewEnumerator1")
      (elif (< _age 30.0)
        (set `self.CurrentStage` "NewEnumerator2")
        (else
          (set `self.CurrentStage` "NewEnumerator3")))))
  (switch `/Game/Farm/Animals/E_GrowthStages` (`self.CurrentStage`)
    (:`NewEnumerator0`
      (`SceneComponent.SetRelativeScale3D` _capsulecomponent (0.4 0.4 0.4)))
    (:`NewEnumerator1`
      (`SceneComponent.SetRelativeScale3D` _capsulecomponent (0.7 0.7 0.7)))
    (:`NewEnumerator2`
      (`SceneComponent.SetRelativeScale3D` _capsulecomponent (1.0 1.0 1.0)))
    (:`NewEnumerator3`
      (`SceneComponent.SetRelativeScale3D` _capsulecomponent (1.0 1.0 1.0)))))

(fn `UserConstructionScript`)